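; Base pickup item actor that shows a prompt widget while looked at and disappears when interacted with.
; StartLooking and StopLooking toggle the Widget component's visibility through SetWidgetActive, which BeginPlay calls to hide it initially.
; The StartInteract override runs the parent logic, destroys the actor, then returns the parent's interaction info and result.
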(event Custom|SetWidgetActive
  (params (IsActive :type Boolean))
  (Development|SetHiddeninGame (Variables|Default|GetWidget) (not IsActive) false))

(event EventBeginPlay
  (CallFunction|SetWidgetActive false))

(event EventStartLooking
  (params (Component :type Interactable%20Component%20Object%20Reference))
  (CallFunction|SetWidgetActive true))

(event EventStopLooking
  (params (Component :type Interactable%20Component%20Object%20Reference))
  (CallFunction|SetWidgetActive false))

(fn ConstructionScript)

(fn StartInteract
  (params (Component :type Interactable%20Component%20Object%20Reference))
  (bind (_interactioninfo _returnvalue) (|CallParentFunction Component))
  (Actor|DestroyActor)
  (return _interactioninfo _returnvalue))