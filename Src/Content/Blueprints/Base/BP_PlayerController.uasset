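; Base player controller that sets up the layered UI for the local player.
; On BeginPlay, the local controller creates the UI manager and pushes the player HUD, while the authority hook is still empty.
; Input actions open the player tabs and main menu, each added asynchronously to the UI layer and initialized with the controller.
; Interaction and inventory event bindings are present but unconnected.
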(event Custom|BeginPlayAsLocalPlayer
  ;[0.15 0.15 0.15 0.5] UI Manager + Player HUD Init
  (bind _returnvalue (UserInterface|CreateWidget "/Game/Blueprints/UI/W_UIManager.W_UIManager_C" self))
  (UserInterface|Viewport|AddtoViewport _returnvalue 0)
  (bind _newwidget (|AddWidgettoLayerAsync "/Game/Blueprints/UI/PlayerHUD/WW_PlayerHUD.WW_PlayerHUD_C" "(TagName=\"LayeredUI.UILayer\")")
    (:Success
      (bind _asww_player_hud (Utilities|Casting|CastToWW_PlayerHUD (.widget _newwidget)))
      (Default|Init _asww_player_hud self))))

(event Custom|BeginPlayAuthority)

(event Input|EnhancedActionEvents|EnhancedInputActionIA_PlayerTabs
  (params (ActionValue :type Boolean) (ElapsedSeconds :type Float%20%28double-precision%29) (TriggeredSeconds :type Float%20%28double-precision%29) (InputAction :type Input%20Action%20Object%20Reference :default "/Game/Input/IA_PlayerTabs.IA_PlayerTabs"))
  ;[0.15 0.15 0.15 0.5] Player UI Tabs
  (:Started
    (bind _newwidget (|AddWidgettoLayerAsync "/Game/Blueprints/UI/PlayerTabs/WW_PlayerTabs.WW_PlayerTabs_C" "(TagName=\"LayeredUI.UILayer\")")
      (:Success
        (bind _asww_player_tabs (Utilities|Casting|CastToWW_PlayerTabs (.widget _newwidget)))
        (Default|Init _asww_player_tabs self)))))

(event Input|EnhancedActionEvents|EnhancedInputActionIA_MainMenu
  (params (ActionValue :type Boolean) (ElapsedSeconds :type Float%20%28double-precision%29) (TriggeredSeconds :type Float%20%28double-precision%29) (InputAction :type Input%20Action%20Object%20Reference :default "/Game/Input/IA_MainMenu.IA_MainMenu"))
  ;[0.15 0.15 0.15 0.5] Main Menu
  (:Started
    (bind _newwidget (|AddWidgettoLayerAsync "/Game/Blueprints/UI/MainMenu/WW_MainMenu.WW_MainMenu_C" "(TagName=\"LayeredUI.UILayer\")")
      (:Success
        (bind _asww_main_menu (Utilities|Casting|CastToWW_MainMenu (.widget _newwidget)))
        (Default|Init _asww_main_menu self)))))

(event EventBeginPlay
  (Utilities|FlowControl|Sequence
    (:then_0
      ;[0.15 0.15 0.15 0.5] Local
      (if (Pawn|IsLocalPlayerController)
        (CallFunction|BeginPlayasLocalPlayer)))
    (:then_1
      ;[0.15 0.15 0.15 0.5] Authority
      (Networking|SwitchHasAuthority
        (:Authority
          (CallFunction|BeginPlayAuthority))))))

(fn ConstructionScript)